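; Lockable elevator door for puzzle interaction: two panels slide apart or together on a timeline, with a ding and positional sounds, and it supplies interaction prompt text.
; Interaction toggles an unlocked door; a locked one checks the player's Keys against DoorkeyID, testing only the element left after the loop completes.
; A match unlocks it and opens after the unlock sound; otherwise the right panel shakes and a voice line plays.
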(event Custom|Check%20for%20Key
  ;[0.7529 0.2831 0.05613 0.502] Check for key
  (for _array_element (Variables|/Game/FirstPerson/Blueprints/BP_FirstPersonCharacter.BP_FirstPersonCharacter_C|GetKeys (Variables|Default|GetPlayer%20Ref))
    _)
  (if (Utilities|Enum|Equal(Enum) _array_element (Variables|Default|GetDoorkeyID))
    (CallFunction|UnlockDoor)
    (else
      (CallFunction|ShakeDoor)
      (Audio|PlaySound2D "/Game/Uploads/Audio/Voice_lines/endvoicedialouge.endvoicedialouge" 1.0 1.0 0.0 0 0))))

(event Custom|Shake%20Door
  ;[0.7529 0.2831 0.05613 0.502] Shake door
  (bind _alpha (Timeline|Shake%20Door%20Timeline PlayFromStart)
    (:Update
      (Transformation|SetRelativeRotation (Variables|Default|GetRight) (Math|Rotator|MakeRotator 0.0 0.0 _alpha) false false))))

(event Custom|Unlock%20Door
  (bind _unlock_sound (Variables|Default|GetUnlock%20Sound))
  ;[0.7529 0.2831 0.05613 0.502] Unlock door
  (Variables|Default|SetisLocked? false)
  (Audio|PlaySoundatLocation _unlock_sound (Transformation|GetWorldLocation (Variables|Default|GetRight)) "0, 0, 0" 1.0 1.0 0.0 0 0 0 0)
  (Utilities|FlowControl|Delay (Variables|/Script/Engine.SoundBase|GetDuration _unlock_sound))
  (CallFunction|Open/closeDoor))

(event Custom|Open/closeDoor
  ;[0.7529 0.2831 0.05613 0.502] open/close door
  (CallFunction|Sounds)
  (Audio|PlaySound2D "/Game/Uploads/Audio/Elevatording.Elevatording" 1.0 1.0 0.0 0 0)
  (if (Variables|Default|GetIs%20Closed?)
    (Variables|Default|SetIs%20Closed? false)
    (bind _openalpha (Timeline|Open/close%20Timeline Play)
      (:Update
        (Transformation|SetRelativeLocation (Variables|Default|GetLeft) (Math|Vector|MakeVector (Math|Float|Lerp -8e+01 -1.7e+02 _openalpha) 0.0 282.0) false false)
        (Transformation|SetRelativeLocation (Variables|Default|GetRight) (Math|Vector|MakeVector (Math|Float|Lerp 74.0 174.0 _openalpha) 0.0 0.0) false false)))
    (else
      (Variables|Default|SetIs%20Closed? true)
      (Timeline|Open/close%20Timeline Reverse))))

(event EventBeginPlay
  ;[0.7529 0.2831 0.05613 0.502] relative pos to door
  (bind _asbp_first_person_character (Utilities|Casting|CastToBP_FirstPersonCharacter (Game|GetPlayerCharacter 0)))
  (Variables|Default|SetPlayer%20Ref _asbp_first_person_character))

(event Collision|EventActorBeginOverlap
  (params (OtherActor :type Actor%20Object%20Reference)))

(event EventTick
  (params (DeltaSeconds :type Float%20%28single-precision%29)))

(event EventInteraction
  (params (Componet :type Primitive%20Component%20Object%20Reference))
  ;[0.7529 0.2831 0.05613 0.502] interaction
  (if (Variables|Default|GetisLocked?)
    (CallFunction|CheckforKey)
    (else
      (CallFunction|Open/closeDoor))))

(fn ConstructionScript)

(fn Sounds
  (bind _right (Variables|Default|GetRight))
  (bind _returnvalue (Transformation|GetWorldLocation _right))
  (if (Variables|Default|GetisLocked?)
    ;[0.15 0.01328 0.01328 0.5] Locked  Sound
    (Audio|PlaySoundatLocation (Variables|Default|GetLocked%20Sound) _returnvalue "0, 0, 0" 1.0 1.0 0.0 0 0 0 0)
    (elif (Variables|Default|GetIs%20Closed?)
      ;[0.15 0.07022 0.01482 0.5] open sound
      (Audio|PlaySoundatLocation (Variables|Default|GetOpen%20Sound) _returnvalue "0, 0, 0" 1.0 1.0 0.0 0 0 0 0)
      (else
        ;[0.15 0.1245 0.01916 0.5] Close Sound
        (Audio|PlaySoundatLocation (Variables|Default|GetClose%20Sound) _returnvalue "0, 0, 0" 1.0 1.0 0.0 0 0 0 0)))))

(fn SendOutNotification
  (params (Component :type Primitive%20Component%20Object%20Reference))
  (return (Variables|Default|GetInteractionText)))