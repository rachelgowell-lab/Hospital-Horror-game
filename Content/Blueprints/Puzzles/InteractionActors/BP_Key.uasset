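; BP_Key is a collectible key actor that the player picks up through interaction.
; On BeginPlay it caches the BP_FirstPersonCharacter, and on Interaction it adds its KeyID to that character, plays a collection sound and destroys itself after a short delay.
; The construction script applies the configurable KeyMesh, and SendOutNotification returns the key's interaction text.
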(event EventBeginPlay
  ;[0.15 0.15 0.15 0.5] c
  (bind _asbp_first_person_character (Utilities|Casting|CastToBP_FirstPersonCharacter (Game|GetPlayerCharacter 0)))
  (Variables|Default|SetPlayer%20ref _asbp_first_person_character))

(event Collision|EventActorBeginOverlap
  (params (OtherActor :type Actor%20Object%20Reference)))

(event EventTick
  (params (DeltaSeconds :type Float%20%28single-precision%29)))

(event EventInteraction
  (params (Componet :type Primitive%20Component%20Object%20Reference))
  ;[0.15 0.15 0.15 0.5] Player Interaction
  (Default|AddKeys (Variables|Default|GetPlayer%20ref) (Variables|Default|GetKeyID))
  (Audio|PlaySound2D (Variables|Default|GetkeyCollectionAudio) 1.0 1.0 0.0 0 0)
  (Utilities|FlowControl|Delay 0.2)
  (Actor|DestroyActor))

(fn ConstructionScript
  (Components|StaticMesh|SetStaticMesh (Variables|Default|GetStaticMesh) (Variables|Default|GetKey%20Mesh)))

(fn SendOutNotification
  (params (Component :type Primitive%20Component%20Object%20Reference))
  (return (Variables|Default|GetInteractionText)))