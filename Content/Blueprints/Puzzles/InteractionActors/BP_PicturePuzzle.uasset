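; BP_PicturePuzzle is an interactable puzzle picture that the player rotates to reach an answer position.
; Each interaction plays a sound and a timeline that lerps the picture's pitch by 90 degrees, ignoring input mid-rotation.
; When finished, it increments a position counter, without wrapping, and compares it to the answer.
; A match locks the puzzle, plays a success sound and calls the completion dispatcher.
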(event Custom|Rotate%20Painting
  ;[0.15 0.15 0.15 0.5] If moving, dont play anim again
  (if (not (Variables|Default|GetFrameMoving))
    (Variables|Default|SetFrameMoving true)
    (Audio|PlaySound2D "/Game/Uploads/Audio/Woosh.Woosh" 1.0 1.0 0.0 0 0)
    (bind _rotationalpha (Timeline|Painting%20Rotation PlayFromStart)
      (:Update
        (Transformation|SetRelativeRotation (Variables|Default|GetPicture) (Math|Rotator|MakeRotator 0.0 (Math|Float|Lerp (.pitch (Variables|Default|GetStartingRoationframe)) (- (.pitch (Variables|Default|GetStartingRoationframe)) 9e+01) _rotationalpha) 0.0) false false))
      (:Finished
        (Variables|Default|SetStartingRoationframe (Math|Rotator|MakeRotator 0.0 (Math|Float|Lerp (.pitch (Variables|Default|GetStartingRoationframe)) (- (.pitch (Variables|Default|GetStartingRoationframe)) 9e+01) _rotationalpha) 0.0))
        (Variables|Default|SetFrameMoving false)
        (bind _result (Math|Integer|IncrementInt (Variables|Default|GetFramePosition))
          (:%20%20
            (Variables|Default|SetFramePosition _result)
            (if (== (Variables|Default|GetPositionAnswer) (Variables|Default|GetFramePosition))
              (Development|PrintString "puzzle complete" true true "(R=0.000000,G=1.000000,B=0.200067,A=1.000000)")
              (Variables|Default|Setfinalized true)
              (Audio|PlaySound2D "/Game/Uploads/Audio/Voice_lines/HellYead.HellYead" 1.0 1.0 0.0 0 0)
              (Default|CallEVDPuzzleCompleted))))))))

(event EventBeginPlay
  (Variables|Default|SetStartingRoationframe (Variables|/Script/Engine.SceneComponent|GetRelativeRotation (Variables|Default|GetPicture))))

(event EventInteraction
  (params (Componet :type Primitive%20Component%20Object%20Reference))
  (if (not (Variables|Default|Getfinalized))
    (CallFunction|RotatePainting)))

(fn ConstructionScript)

(fn SendOutNotification
  (params (Component :type Primitive%20Component%20Object%20Reference))
  (return (Variables|Default|GetInteractionText)))